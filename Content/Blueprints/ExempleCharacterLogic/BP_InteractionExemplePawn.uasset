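; Example pawn showing how to drive BPC_InteractorComponent to find, select and trigger interactables.
; Tick line-traces from the pawn along camera forward, tracking the focused BPC_InteractibleComponent and toggling its UI.
; F calls the interaction, and mouse wheel scrolling past a threshold changes the selected one.
; PreInteraction pauses searching, prints the action's DT_ExempleInteractionPreLogic message, and fires the required InteractionCallback by timer before searching resumes after a delay.
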(event Custom|PreInteraction
  (params (Action :type Interaction%20Class%20Reference))
  ;[0.314 0.314 0.314] EXEMPLE: Execute custom logic based on executed action before the interaction actually complites
  (Variables|Default|SetbLookForInteractables false)
  ;;[0.0999 0 0.4969] Data Table cuold be used to associate animations, sounds, VFX or messages to specific interactions
  (bind _outrownames (DataTable|GetDataTableRowNames "/InteractionSystem/Blueprints/ExempleCharacterLogic/DT_ExempleInteractionPreLogic.DT_ExempleInteractionPreLogic"))
  (bind _array_element (Utilities|Array|ForEachLoopwithBreak _outrownames :!label _label)
    (:LoopBody
      (bind _returnvalue (Utilities|GetDataTableRow "/InteractionSystem/Blueprints/ExempleCharacterLogic/DT_ExempleInteractionPreLogic.DT_ExempleInteractionPreLogic" _array_element)
        (:then
          (if (== (.Interaction (Utilities|Struct|BreakS_ExempleInteractionPreLogic _returnvalue)) Action)
            (Utilities|FlowControl|Sequence
              (:then_0
                (Development|PrintString (.Message (Utilities|Struct|BreakS_ExempleInteractionPreLogic _returnvalue))))
              (:then_1
                (goto _label Break)))))))
    (:Completed
      ;;[1 0.2 0] InteractionCallback must be called when custom logic has finished
      ;; Will not work otherwise
      (Utilities|Time|SetTimerbyFunctionName (Variables|Default|GetBPC_InteractorComponent) "InteractionCallback" 2.0)
      (Utilities|FlowControl|Delay 3.0)
      (Variables|Default|SetbLookForInteractables true))))

(event EventBeginPlay
  ;[1 0.2 0] Need to subscribe to receive the go ahead from the interaction
  ; Will not work if not subscribed
  (EventDispatchers|BindEventtoOnInteractionConfirmed (Variables|Default|GetBPC_InteractorComponent) (EventDispatchers|CreateEvent :!event Custom|PreInteraction)))

(event Collision|EventActorBeginOverlap
  (params (OtherActor :type Actor%20Object%20Reference)))

(event EventTick
  (params (DeltaSeconds :type Float%20%28single-precision%29))
  (bind _returnvalue (Transformation|GetActorLocation))
  (bind _bpc_interactorcomponent (Variables|Default|GetBPC_InteractorComponent))
  ;[1 1 1] EXEMPLE: Search and keep track of interactables (store focused one and call show/hide User Interface)
  (if (Variables|Default|GetbLookForInteractables)
    (bind (_outhit _returnvalue_2) (Collision|LineTraceByChannel _returnvalue (+ _returnvalue (* (Math|Vector|GetForwardVector (Variables|/Script/Engine.PlayerCameraManager|GetTransformComponent (Game|GetPlayerCameraManager 0))) (Variables|Default|GetInteractionDistance))) "TraceTypeQuery1" false 0 "None"))
    (if _returnvalue_2
      (Utilities|IsValid (Actor|GetComponentbyClass (.HitActor (Collision|BreakHitResult _outhit)) "/InteractionSystem/Blueprints/Components/BPC_InteractibleComponent.BPC_InteractibleComponent_C")
        (:Is%20Valid
          (Utilities|IsValid (Variables|/Script/InteractionSystem.InteractorComponent|GetFocusedInteractible (Variables|Default|GetBPC_InteractorComponent))
            (:Is%20Valid
              (if (!= (Actor|GetComponentbyClass (.HitActor (Collision|BreakHitResult _outhit)) "/InteractionSystem/Blueprints/Components/BPC_InteractibleComponent.BPC_InteractibleComponent_C") (Variables|/Script/InteractionSystem.InteractorComponent|GetFocusedInteractible (Variables|Default|GetBPC_InteractorComponent)))
                (Class|InteractibleComponent|HideUserInterface (Variables|/Script/InteractionSystem.InteractorComponent|GetFocusedInteractible (Variables|Default|GetBPC_InteractorComponent)))
                (bind _output_get (Variables|/Script/InteractionSystem.InteractorComponent|SetFocusedInteractible (Variables|Default|GetBPC_InteractorComponent) (Actor|GetComponentbyClass (.HitActor (Collision|BreakHitResult _outhit)) "/InteractionSystem/Blueprints/Components/BPC_InteractibleComponent.BPC_InteractibleComponent_C")))
                (Class|InteractibleComponent|ShowUserInterface _output_get)))
            (:Is%20Not%20Valid
              (bind _output_get_2 (Variables|/Script/InteractionSystem.InteractorComponent|SetFocusedInteractible (Variables|Default|GetBPC_InteractorComponent) (Actor|GetComponentbyClass (.HitActor (Collision|BreakHitResult _outhit)) "/InteractionSystem/Blueprints/Components/BPC_InteractibleComponent.BPC_InteractibleComponent_C")))
              (Class|InteractibleComponent|ShowUserInterface _output_get_2))))
        (:Is%20Not%20Valid
          (Utilities|IsValid (Variables|/Script/InteractionSystem.InteractorComponent|GetFocusedInteractible _bpc_interactorcomponent) :!label _label
            (:Is%20Valid
              (Class|InteractibleComponent|HideUserInterface (Variables|/Script/InteractionSystem.InteractorComponent|GetFocusedInteractible _bpc_interactorcomponent))
              (Variables|/Script/InteractionSystem.InteractorComponent|SetFocusedInteractible _bpc_interactorcomponent 0)))))
      (else
        (goto _label)))))

(event Input|MouseEvents|MouseWheelAxis
  (params (AxisValue :type Float%20%28single-precision%29))
  (bind _bpc_interactorcomponent (Variables|Default|GetBPC_InteractorComponent))
  (bind _focusedinteractible (Variables|/Script/InteractionSystem.InteractorComponent|GetFocusedInteractible _bpc_interactorcomponent))
  ;[1 1 1] EXEMPLE: Change the selected interaction in focused interactable
  (Utilities|IsValid _focusedinteractible
    (:Is%20Valid
      (bind _output_get (Variables|Default|SetScrollAxisValue (+ (* AxisValue -1.0) (Variables|Default|GetScrollAxisValue))))
      (if (> (Math|Float|Absolute(Float) _output_get) (Variables|Default|GetScrollThreshold))
        (Class|InteractibleComponent|ChangeSelectedInteraction _focusedinteractible (Math|Integer|SelectInt 1 -1 (> (Variables|Default|GetScrollAxisValue) 0.0)))
        (Variables|Default|SetScrollAxisValue 0.0)))))

(event Input|KeyboardEvents|F
  (params (Key :type Key%20Structure :default "None"))
  ;[1 1 1] EXEMPLE: Call interaction through component
  (:Pressed
    (Class|InteractorComponent|CallInteraction (Variables|Default|GetBPC_InteractorComponent))))

(fn ConstructionScript)