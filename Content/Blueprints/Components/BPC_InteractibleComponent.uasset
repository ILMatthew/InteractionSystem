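; Interactible component that shows an interaction wheel on its owning actor and keeps it in sync with the selected action.
; Showing builds the wheel from the available actions' class defaults in a runtime-created, screen-space widget component, retrying by timer while an old one still exists.
; Hiding cancels any queued show, plays the close, then destroys the widget after a delay.
; Selection and error overrides call the parent, then update the wheel.
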(event EventBeginPlay)

(event EventTick
  (params (DeltaSeconds :type Float%20%28single-precision%29)))

(event EventShowUserInterface
  (bind _avaiableactions (Variables|Default|GetAvaiableActions))
  ;[1 1 1] Add Custom logic to control User Interface
  ;;[0.1251 1 0] Crates and show User Interface
  (Utilities|IsValid (Variables|UI|GetWidgetComp)
    (:Is%20Valid
      (bind _returnvalue (Utilities|Time|SetTimerbyEvent (delegate EventShowUserInterface) 1.0))
      (Variables|UI|SetShowUserInterfaceQueue _returnvalue))
    (:Is%20Not%20Valid
      (Class|InteractibleComponent|ChangeSelectedInteraction)
      (bind _returnvalue_2 (UserInterface|CreateWidget "/InteractionSystem/UI/WBP_InteractionWheel.WBP_InteractionWheel_C"))
      (bind _output_get (Variables|UI|SetInteractionWheel _returnvalue_2))
      (Variables|/InteractionSystem/UI/WBP_InteractionWheel.WBP_InteractionWheel_C|SetInteractionsNum _output_get (Utilities|Array|Length _avaiableactions))
      (for _array_element _avaiableactions
        (Utilities|Array|Add (Variables|/InteractionSystem/UI/WBP_InteractionWheel.WBP_InteractionWheel_C|GetActions _output_get) (Utilities|GetClassDefaults _array_element)))
      (Default|UpdateOptionWheel _output_get)
      (bind _returnvalue_3 (Game|AddComponentbyClass (Components|GetOwner) "/Script/UMG.WidgetComponent" false))
      (bind _output_get_2 (Variables|UI|SetWidgetComp _returnvalue_3))
      (Class|WidgetComponent|SetWidgetSpace _output_get_2 "Screen")
      (UserInterface|SetWidget _output_get_2 (Variables|UI|GetInteractionWheel))
      (Collision|SetCollisionEnabled _output_get_2 "NoCollision")
      (Widget|SetRenderOpacity (Variables|UI|GetInteractionWheel) 1.0)
      (Default|OpenWheel (Variables|UI|GetInteractionWheel)))))

(event EventHideUserInterface
  (bind _interactionwheel (Variables|UI|GetInteractionWheel))
  (bind _widgetcomp (Variables|UI|GetWidgetComp))
  ;[1 1 1] Add Custom logic to control User Interface
  ;;[1 0 0.01377] Hide and Destroy User Interface
  (Utilities|Time|ClearandInvalidateTimerbyHandle (Variables|UI|GetShowUserInterfaceQueue))
  (Utilities|IsValid _widgetcomp
    (:Is%20Valid
      (Default|CloseWheel _interactionwheel)
      (Utilities|FlowControl|Delay (Class|WidgetAnimation|GetEndTime (Variables|/InteractionSystem/UI/WBP_InteractionWheel.WBP_InteractionWheel_C|GetOpenSelection _interactionwheel)))
      (Components|DestroyComponent _widgetcomp (Components|GetOwner))
      (Widget|RemovefromParent (Variables|UI|GetInteractionWheel)))))

(event EventChangeSelectedInteraction
  (params (indexOffset :type Integer))
  ;[1 1 1] Add Custom logic to control User Interface
  ;;[0 0.4514 1] Change selected interaction and show it on User Interface
  (|CallParentFunction indexOffset)
  (Utilities|IsValid (Variables|UI|GetWidgetComp)
    (:Is%20Valid
      (Default|SelectOption (Variables|UI|GetInteractionWheel) (Variables|Default|GetcurrentSelection)))))

(event EventSelectInteraction
  (params (interactionIndex :type Integer))
  ;[1 1 1] Add Custom logic to control User Interface
  ;;[0 0.4514 1] Change selected interaction and show it on User Interface
  (|CallParentFunction interactionIndex)
  (Utilities|IsValid (Variables|UI|GetWidgetComp)
    (:Is%20Valid
      (Default|SelectOption (Variables|UI|GetInteractionWheel) (Variables|Default|GetcurrentSelection)))))

(event EventDisplayError
  (params (Message :type Text%20%28by%20ref%29))
  (|CallParentFunction Message)
  (Utilities|IsValid (Variables|UI|GetWidgetComp)
    (:Is%20Valid
      (Default|DisplayError (Variables|UI|GetInteractionWheel) Message))))