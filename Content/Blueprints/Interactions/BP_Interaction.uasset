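; BP_Interaction is a skeleton interaction Blueprint with placeholder hooks for check and interaction logic.
; CheckInteraction calls its parent, then runs CustomCheck and, on success, passes its own class to the caller's InteractionGoAhead.
; InteractionLogic runs CustomLogic before calling the parent implementation.
; Both hooks are stubs: CustomCheck always returns false, so this Blueprint's go-ahead never fires as written, and CustomLogic is empty.
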(event EventCheckInteraction
  (params (called :type Interactible%20Component%20Object%20Reference%20%28by%20ref%29) (caller :type Interactor%20Component%20Object%20Reference%20%28by%20ref%29))
  (|CallParentFunction called caller)
  ;[1 1 1] Add Check logic
  (bind _interactionsucceded (CallFunction|CustomCheck))
  (if _interactionsucceded
    (Class|InteractorComponent|InteractionGoAhead (Variables|Default|GetCallerObject) (Utilities|GetClass self))))

(event EventInteractionLogic
  ;[1 1 1] Add Interaction logic
  (CallFunction|CustomLogic)
  (|CallParentFunction))

(fn CustomCheck
  (return false))

(fn CustomLogic)